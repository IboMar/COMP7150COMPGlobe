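; Globe actor that shows six named location markers (continents, plus Ireland) with UI labels and can be grabbed.
; On BeginPlay it attaches a LocationUI widget component to each location point and passes that point's name to the widget.
; Tick rotates every point to face the player pawn, billboarding the labels.
; Grabbing adds the GrabComponent's world rotation to the globe once per grab event.
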(event `self.ReceiveBeginPlay`
  (bind _array (`|MakeArray` (`self.Asia`) (`self.NorthAmerica`) (`self.Europe`) (`self.Australia`) (`self.Ireland`) (`self.SouthAmerica`)))
  ;[1 1 1] AttachWidget button to each point
  (set `self.ListOfLocations` _array)
  (for _array_element _array
    (bind _returnvalue (`AddComponent|NODE_AddWidgetComponent-0` :`RelativeTransform` (`KismetMathLibrary.MakeTransform` (100.0 0.0 0.0))))
    (`SceneComponent.K2_AttachToComponent` _returnvalue _array_element "None" "SnapToTarget" "KeepWorld" "KeepRelative" false)
    (bind _aslocation_ui (cast `/Game/Assignment/blueprint/widget/LocationUI` (`WidgetComponent.GetWidget` _returnvalue)))
    (`/Game/Assignment/blueprint/widget/LocationUI.SetLocation` _aslocation_ui (`KismetStringLibrary.Conv_ObjectToString` _array_element))))

(event `self.GrabComponent.OnGrabbed`
  (`SceneComponent.K2_AddWorldRotation` (`self.Globe`) (`SceneComponent.K2_GetComponentRotation` (`self.GrabComponent`)) false false))

(event `self.ReceiveTick`
  (params (DeltaSeconds :type "Float (single-precision)"))
  (for _array_element (`self.ListOfLocations`)
    (`SceneComponent.K2_SetWorldRotation` _array_element (`KismetMathLibrary.FindLookAtRotation` (`SceneComponent.K2_GetComponentLocation` _array_element) (`self.K2_GetActorLocation` (`GameplayStatics.GetPlayerPawn` 0))) false false)))

(fn `UserConstructionScript`)